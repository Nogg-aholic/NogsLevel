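; BP_Edible_Parent is, by its name, the base Blueprint for edible pickup items.
; On pickup it runs the parent class's OnPickup, then, on the authority only, sets NumItems to NumToGive.
; All other pickup behavior comes from the parent class, as BeginPlay, overlap and Tick are disabled stubs and the construction script only calls its parent.
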(event EventBeginPlay
  (|CallParentFunction) ; This node is disabled and will not be called.\nDrag off pins to build functionality.
)

(event Collision|EventActorBeginOverlap
  (params (OtherActor :type Actor%20Object%20Reference))
  (|CallParentFunction OtherActor) ; This node is disabled and will not be called.\nDrag off pins to build functionality.
)

(event EventTick
  (params (DeltaSeconds :type Float%20%28single-precision%29))
  (|CallParentFunction DeltaSeconds) ; This node is disabled and will not be called.\nDrag off pins to build functionality.
)

(event EventOnPickup
  (params (byCharacter :type FG%20Character%20Player%20Object%20Reference))
  (|CallParentFunction byCharacter)
  (Networking|SwitchHasAuthority
    (:Authority
      (Class|FGItemPickup|SetNumItems (Variables|Default|GetNumToGive)))))

(fn ConstructionScript
  (|CallParentFunction))