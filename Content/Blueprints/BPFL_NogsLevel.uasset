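; Blueprint function library for the Nogs level that applies NogsLevelConfig options for cheats, sky lighting and water.
; It copies NoCost and NoPower to the game state and toggles BP_NogSkyActor visibility and ticking by CustomLight.
; SetupWater enlarges a water volume for WaterWorld and swaps materials on its attached meshes.
; FixWaterExtractorPlacement edits the too-shallow disqualifier's class default object to make it soft.
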(fn SetCheatVariables
  (bind _returnvalue (Class|RuntimeBlueprintFunctionLibrary|ToConfigProperty(ModConfiguration) "/NogsLevel/NogsLevelConfig.NogsLevelConfig_C"))
  (bind _asbp_config_property_section (Utilities|Casting|CastToBP_ConfigPropertySection _returnvalue))
  (bind _asbp_game_state (Utilities|Casting|CastToBP_GameState (Game|GetGameState)))
  (Class|FGGameState|SetCheatNoCost _asbp_game_state (Class|RuntimeBlueprintFunctionLibrary|ToBoolean(ConfigProperty) (Class|RuntimeBlueprintFunctionLibrary|ToConfigProperty(ConfigPropertySection) _asbp_config_property_section "NoCost")))
  (Class|FGGameState|SetCheatNoPower _asbp_game_state (Class|RuntimeBlueprintFunctionLibrary|ToBoolean(ConfigProperty) (Class|RuntimeBlueprintFunctionLibrary|ToConfigProperty(ConfigPropertySection) _asbp_config_property_section "NoPower"))))

(fn DestroyLights
  (bind _returnvalue (Class|RuntimeBlueprintFunctionLibrary|ToConfigProperty(ModConfiguration) "/NogsLevel/NogsLevelConfig.NogsLevelConfig_C"))
  (bind _asbp_config_property_section (Utilities|Casting|CastToBP_ConfigPropertySection _returnvalue))
  (bind _returnvalue_2 (Class|RuntimeBlueprintFunctionLibrary|ToConfigProperty(ConfigPropertySection) _asbp_config_property_section "CustomLight"))
  (bind _returnvalue_3 (Class|RuntimeBlueprintFunctionLibrary|ToBoolean(ConfigProperty) _returnvalue_2))
  (bind _outactors (Actor|GetAllActorsOfClass 0 "/NogsLevel/Blueprints/BP_NogSkyActor.BP_NogSkyActor_C"))
  (for _array_element _outactors
    (Rendering|SetActorHiddenInGame _array_element (not _returnvalue_3))
    (Actor|Tick|SetActorTickEnabled _array_element _returnvalue_3)))

(fn SetupWater
  (if (Class|RuntimeBlueprintFunctionLibrary|ToBoolean(ConfigProperty) (Class|RuntimeBlueprintFunctionLibrary|ToConfigProperty(ConfigPropertySection) (.AsBP%20Config%20Property%20Section (Utilities|Casting|CastToBP_ConfigPropertySection (Class|RuntimeBlueprintFunctionLibrary|ToConfigProperty(ModConfiguration) "/NogsLevel/NogsLevelConfig.NogsLevelConfig_C"))) "WaterWorld"))
    (bind _returnvalue (Actor|GetActorOfClass 0 "/Script/FactoryGame.FGWaterVolume"))
    (Transformation|SetActorScale3D _returnvalue "55.000000,55.000000,1.000000"))
  (for _array_element (Actor|GetAttachedActors _returnvalue true)
    (bind _asstatic_mesh_actor (Utilities|Casting|CastToStaticMeshActor _array_element))
    (if (Utilities|Enum|Equal(Enum) (Utilities|GetDisplayName _array_element) "WaterUnderSide")
      (Rendering|Material|SetMaterial (Variables|/Script/Engine.StaticMeshActor|GetStaticMeshComponent _asstatic_mesh_actor) 0 "/Game/FactoryGame/World/Environment/Water/Material/MI_Water_Translucent.MI_Water_Translucent")
      (else
        ;[1 1 1] TODOU5 need to switch back to the nice custom ocean material eventually
        (Rendering|Material|SetMaterial (Variables|/Script/Engine.StaticMeshActor|GetStaticMeshComponent _asstatic_mesh_actor) 0 "/Game/FactoryGame/World/Environment/Water/Lake/Material/LakeWater_01_Inst.LakeWater_01_Inst")))))

(fn FixWaterExtractorPlacement
  (Variables|/Script/FactoryGame.FGConstructDisqualifier|SetmIsSoftDisqualifier (Class|BlueprintReflectionLibrary|GetClassDefaultObject "/Script/FactoryGame.FGCDResourceIsTooShallow") true) ; Thanks D4rkL0rd
)